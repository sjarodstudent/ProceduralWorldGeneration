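; Procedural building actor that, on BeginPlay, assembles a walled compound from randomly picked static meshes on a CellSize-based grid.
; GenerateOutWalls rings an OutWidth by OutDepth perimeter with wall and corner pieces.
; GenerateCenter reads the Dungeon array of height rows, stacking wall pieces per cell and capping each with a roof.
; SpawnMesh spawns each piece as an attached, movable StaticMeshActor; an older instanced-mesh version remains disconnected in the construction script.
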(event EventBeginPlay
  (CallFunction|GenerateOutWalls)
  (CallFunction|GenerateCenter))

(event Collision|EventActorBeginOverlap
  (params (OtherActor :type Actor%20Object%20Reference)))

(event EventTick
  (params (DeltaSeconds :type Float%20%28single-precision%29)))

(fn ConstructionScript)

(fn SpawnMesh
  (params (NewMesh :type Static%20Mesh%20Object%20Reference) (NewRelativeLocation_X :type Float%20%28double-precision%29) (NewRelativeLocation_Y :type Float%20%28double-precision%29) (New%20Relative%20Location%20Z :type Float%20%28double-precision%29) (New%20Relative%20Rotation%20Z%20%28Yaw%29 :type Float%20%28single-precision%29))
  (bind _returnvalue (Game|SpawnActorfromClass "/Script/Engine.StaticMeshActor" (Math|Transform|MakeTransform "0, 0, 0" "0, 0, 0" "1.000000,1.000000,1.000000") "Undefined" "MultiplyWithRoot" 0 0))
  (Transformation|SetMobility _returnvalue "Movable")
  (Transformation|AttachComponentToComponent _returnvalue (Variables|Default|GetDefaultSceneRoot) "None" "KeepRelative" "KeepRelative" "KeepRelative" true)
  (Transformation|SetActorRelativeLocation _returnvalue (Math|Vector|MakeVector NewRelativeLocation_X NewRelativeLocation_Y New%20Relative%20Location%20Z))
  (Transformation|SetActorRelativeRotation _returnvalue (Math|Rotator|MakeRotator 0.0 0.0 New%20Relative%20Rotation%20Z%20%28Yaw%29))
  (Components|StaticMesh|SetStaticMesh (Variables|/Script/Engine.StaticMeshActor|GetStaticMeshComponent _returnvalue) NewMesh))

(fn GenerateOutWalls
  (bind _cellsize (Variables|Default|GetCellSize))
  (bind _cellsize_2 (Variables|Default|GetCellSize))
  (bind _cellsize_3 (Variables|Default|GetCellSize))
  (bind _cellsize_4 (Variables|Default|GetCellSize))
  (bind _cellsize_5 (Variables|Default|GetCellSize))
  (bind _cellsize_6 (Variables|Default|GetCellSize))
  (bind _cellsize_7 (Variables|Default|GetCellSize))
  (bind _cellsize_8 (Variables|Default|GetCellSize))
  (Utilities|FlowControl|Sequence
    (:then_0
      ;[1 1 1] Out Front
      (for _index (range 0 (- (Variables|Default|GetOut_Width) 1))
        (CallFunction|SpawnMesh (.OutItem (Utilities|Array|Random (Variables|Default|GetOut_Walls))) (+ _cellsize_5 (* _cellsize_5 (Variables|Default|GetOut_Depth))) (- (* _index (* 2.0 _cellsize_5)) (* _cellsize_5 (- (Variables|Default|GetOut_Width) 1))) 0.0 1.8e+02)))
    (:then_1
      ;[1 1 1] Out Back
      (for _index_2 (range 0 (- (Variables|Default|GetOut_Width) 1))
        (CallFunction|SpawnMesh (.OutItem (Utilities|Array|Random (Variables|Default|GetOut_Walls))) (- (+ (* _cellsize_6 (Variables|Default|GetOut_Depth) -1.0 2.0) (* _cellsize_6 (Variables|Default|GetOut_Depth))) _cellsize_6) (- (* _index_2 (* 2.0 _cellsize_6)) (* _cellsize_6 (- (Variables|Default|GetOut_Width) 1))) 0.0 0.0)))
    (:then_2
      ;[1 1 1] Out Left
      (for _index_3 (range 0 (- (Variables|Default|GetOut_Depth) 1))
        (CallFunction|SpawnMesh (.OutItem (Utilities|Array|Random (Variables|Default|GetOut_Walls))) (- (* _index_3 (* 2.0 _cellsize_7)) (* _cellsize_7 (- (Variables|Default|GetOut_Depth) 1))) (- (+ (* _cellsize_7 (Variables|Default|GetOut_Width) -1.0 2.0) (* _cellsize_7 (Variables|Default|GetOut_Width))) _cellsize_7) 0.0 9e+01)))
    (:then_3
      ;[1 1 1] Out Left
      (for _index_4 (range 0 (- (Variables|Default|GetOut_Depth) 1))
        (CallFunction|SpawnMesh (.OutItem (Utilities|Array|Random (Variables|Default|GetOut_Walls))) (- (* _index_4 (* 2.0 _cellsize_4)) (* _cellsize_4 (- (Variables|Default|GetOut_Depth) 1))) (+ _cellsize_4 (* _cellsize_4 (Variables|Default|GetOut_Width))) 0.0 2.7e+02)))
    (:then_4
      ;[1 1 1] Out Corner 1
      (CallFunction|SpawnMesh (.OutItem (Utilities|Array|Random (Variables|Default|GetOut_Corners))) (+ _cellsize_8 (* _cellsize_8 (Variables|Default|GetOut_Depth))) (+ (- (* (- (Variables|Default|GetOut_Width) 1) (* 2.0 _cellsize_8)) (* _cellsize_8 (- (Variables|Default|GetOut_Width) 1))) (* _cellsize_8 2.0)) 0.0 9e+01))
    (:then_5
      ;[1 1 1] Out Corner 1
      (CallFunction|SpawnMesh (.OutItem (Utilities|Array|Random (Variables|Default|GetOut_Corners))) (+ _cellsize (* _cellsize (Variables|Default|GetOut_Depth))) (- (- 0.0 (* _cellsize (- (Variables|Default|GetOut_Width) 1))) (* _cellsize 2.0)) 0.0 0.0))
    (:then_6
      ;[1 1 1] Out Corner 1
      (CallFunction|SpawnMesh (.OutItem (Utilities|Array|Random (Variables|Default|GetOut_Corners))) (- (- 0.0 (* _cellsize_2 (- (Variables|Default|GetOut_Depth) 1))) (* _cellsize_2 2.0)) (- (- 0.0 (* _cellsize_2 (- (Variables|Default|GetOut_Width) 1))) (* _cellsize_2 2.0)) 0.0 2.7e+02))
    (:then_7
      ;[1 1 1] Out Corner 1
      (CallFunction|SpawnMesh (.OutItem (Utilities|Array|Random (Variables|Default|GetOut_Corners))) (- (- 0.0 (* _cellsize_3 (- (Variables|Default|GetOut_Depth) 1))) (* _cellsize_3 2.0)) (+ _cellsize_3 (* _cellsize_3 (Variables|Default|GetOut_Width))) 0.0 1.8e+02))))

(fn GenerateCenter
  (bind _dungeon (Variables|Default|GetDungeon))
  (bind _cellsize (Variables|Default|GetCellSize))
  (bind _cellsize_2 (Variables|Default|GetCellSize))
  (for (_array_element _array_index) _dungeon
    (for (_array_element_2 _array_index_2) (Utilities|Struct|BreakLine _array_element)
      (for _index (range 0 _array_element_2)
        (if (< _index _array_element_2)
          (CallFunction|SpawnMesh (.OutItem (Utilities|Array|Random (Variables|Default|GetDungeonWalls))) (- (* _array_index (* 2.0 _cellsize)) (* _cellsize (- (Utilities|Array|Length _dungeon) 1))) (- (* _array_index_2 (* 2.0 _cellsize_2)) (* _cellsize_2 (- (Utilities|Array|Length (Utilities|Struct|BreakLine _array_element)) 1))) (* _index (* 2.0 (Variables|Default|GetCellSize))) 0.0)
          (else
            (CallFunction|SpawnMesh (.OutItem (Utilities|Array|Random (Variables|Default|GetDungeonRoofs))) (- (* _array_index (* 2.0 _cellsize)) (* _cellsize (- (Utilities|Array|Length _dungeon) 1))) (- (* _array_index_2 (* 2.0 _cellsize_2)) (* _cellsize_2 (- (Utilities|Array|Length (Utilities|Struct|BreakLine _array_element)) 1))) (* _index (* 2.0 (Variables|Default|GetCellSize))) 0.0)))))))